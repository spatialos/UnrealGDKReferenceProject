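; BP_NPC_Controller is the AI controller for NPCs, running a wander-and-shoot behavior tree on the authority.
; A looping timer, also started on AuthorityGained, passes AI perception and the current target to EvaluateTargets and writes the result to the blackboard.
; Sight is enabled after a short startup delay, and the perception update event is unused.
; Death unpossesses the pawn, clears the alive flag and destroys the controller after a delay.
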(event `self.ReceiveBeginPlay`
  (`/Engine/EditorBlueprintResources/ActorMacros.Switch Has Authority`
    (:`Authority`
      (`|ExecutionSequence`
        (:`then_0`
          (`self.UseBlackboard` "/Game/AI/BB_NPC.BB_NPC")
          (`self.RunBehaviorTree` "/Game/AI/BT_WanderAndShoot.BT_WanderAndShoot")
          (`BlackboardComponent.SetValueAsBool` (`self.Blackboard`) (`self.IsAliveKey`) true)
          (`KismetSystemLibrary.K2_SetTimerDelegate` (delegate `EvaluateTargets`) 0.2 true :!label _label))
        (:`then_1`
          (`KismetSystemLibrary.Delay` 2.0)
          (`AIPerceptionComponent.SetSenseEnabled` (`self.AIPerception`) "/Script/AIModule.AISense_Sight" true))))))

(event `self.AIPerception.OnPerceptionUpdated`
  (params (UpdatedActors :type "Array of Actor Object Reference (by ref)")))

(event `self.ReceiveAuthorityGained`
  (goto _label))

(event `EvaluateTargets`
  (bind _blackboard (`self.Blackboard`))
  (bind _targetkey (`self.TargetKey`))
  (bind _target (`/Game/Controllers/Components/BPL_TargetSelection.EvaluateTargets` (`self.AIPerception`) (`self.CurrentTarget`)))
  (bind _output_get (set `self.CurrentTarget` _target))
  (`/Engine/EditorBlueprintResources/StandardMacros.IsValid` _output_get
    (:`Is Valid`
      (`BlackboardComponent.SetValueAsObject` _blackboard _targetkey (`self.CurrentTarget`)))
    (:`Is Not Valid`
      (`BlackboardComponent.ClearValue` _blackboard _targetkey))))

(event `self.ControllerEvents.DeathEvent`
  (params (Controller :type "Controller Object Reference"))
  (`self.UnPossess`)
  (`BlackboardComponent.SetValueAsBool` (`self.Blackboard`) (`self.IsAliveKey`) false)
  (`KismetSystemLibrary.Delay` 1.0)
  (`self.K2_DestroyActor`))

(fn `UserConstructionScript`)