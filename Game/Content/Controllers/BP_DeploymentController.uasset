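; BP_DeploymentController is the player controller for the deployment screen in CorridorShooter, with the mouse cursor shown.
; On BeginPlay it polls on a short delay loop until its PartySystem is valid, then passes it the player identity stored in the game instance.
; A debug Space Bar binding skips the login flow by calling OnLoginComplete on the deployments HUD.
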(event `self.ReceiveBeginPlay`
  (bind _partysystem (`self.PartySystem`))
  (`parent.ReceiveBeginPlay`)
  (set `self.bShowMouseCursor` true)
  (bind _ascorridor_shooter_game_instance (cast `CorridorShooterGameInstance` (`GameplayStatics.GetGameInstance`)))
  (`/Engine/EditorBlueprintResources/StandardMacros.IsValid` _partysystem :!label _label
    (:`Is Valid`
      (`PartySystem.InformOfPlayerIdentity` _partysystem (`CorridorShooterGameInstance.PlayerIdentity` _ascorridor_shooter_game_instance)))
    (:`Is Not Valid`
      (`KismetSystemLibrary.Delay` 0.2)
      (goto _label))))

(event `Key|SpaceBar`
  (params (Key :type "Key Structure"))
  ;[1 1 1] Debug spacebar to skip login flow
  (:`Pressed`
    (bind _asbp_hud_deployments (cast `/Game/UI/Blueprints/Deployments/BP_HUD_Deployments` (`self.GetHUD`)))
    (`/Game/UI/Blueprints/Deployments/BP_HUD_Deployments.OnLoginComplete` _asbp_hud_deployments)))

(fn `UserConstructionScript`)