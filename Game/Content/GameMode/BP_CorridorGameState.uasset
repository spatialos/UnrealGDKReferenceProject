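; Game state for the Corridor mode, wiring components together to run a squad match from lobby through phased zones to post-game.
; Publisher events feed scoring, player counting, squad tracking and team spawning; player count drives the lobby timer, which starts the match.
; On authority, each new zone restarts the match timer until the final phase; timer expiry advances the phase and disables respawning.
; Zone starts also check for a last-squad win in the final phase.
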(event `self.ScorePublisher.KillEvent`
  (params (Killer :type String) (Victim :type String))
  ;[1 1 1] Publish Scores
  (`DeathmatchScoreComponent.RecordKill` (`self.DeathmatchScore`) Killer Victim))

(event `self.PlayerPublisher.PlayerEvent`
  (params (PlayerState :type "PlayerState Object Reference") (Progress :type "EPlayerProgress Enum" :default "Connected"))
  ;[1 1 1] Listen to player events
  (`PlayerCountingComponent.PlayerEvent` (`self.PlayerCounting`) PlayerState Progress)
  (if (`|EnumEquality` Progress "InGame")
    (`/Game/GameMode/Components/SquadTrackingComponent.RegisterInGamePlayer` (`self.SquadTrackingComponent`) PlayerState)
    (`DeathmatchScoreComponent.RecordNewPlayer` (`self.DeathmatchScore`) PlayerState)))

(event `self.ScorePublisher.DeathEvent`
  (params (VictimState :type "PlayerState Object Reference"))
  ;[1 1 1] Publish Scores
  (`/Game/GameMode/Components/SquadTrackingComponent.RegisterDeath` (`self.SquadTrackingComponent`) VictimState))

(event `self.PlayerCounting.PlayerCountEvent`
  (params (PlayerCount :type Integer))
  ;[1 1 1] Start Lobby Countdown
  (`LobbyTimerComponent.ServerInformOfPlayerCount` (`self.LobbyTimer`) PlayerCount))

(event `self.LobbyTimer.OnTimerFinished`
  ;[1 1 1] Start Match After Lobby
  (`MatchStateComponent.SetMatchState` (`self.MatchState`) "InGame")
  (`/Game/GameMode/Components/PhaseBasedMapComponent.StartGame` (`self.PhaseBasedMapComponent`))
  (`MatchStateComponent.SetMatchState` (`self.MatchState`) "InGame"))

(event `self.PhaseBasedMapComponent.ZoneBegun`
  (params (NewZone :type Integer))
  (bind _phasebasedmapcomponent (`self.PhaseBasedMapComponent`))
  (bind _matchtimer (`self.MatchTimer`))
  (bind _output_phaselength (break `/Game/GameMode/Components/PhaseEntry` (`|GetArrayItem` (`/Game/GameMode/Components/PhaseData.PhaseData` (`/Game/GameMode/Components/PhaseBasedMapComponent.PhaseData` _phasebasedmapcomponent)) NewZone)))
  ;[1 1 1] Finish Timer
  (`/Engine/EditorBlueprintResources/ActorMacros.Switch Has Authority`
    (:`Authority`
      (`self.EvaluateWinCondition`)
      (if (and (not (`/Game/GameMode/Components/PhaseBasedMapComponent.IsInFinalPhase` _phasebasedmapcomponent)) (`/Game/GameMode/Components/PhaseBasedMapComponent.HasPhaseData` _phasebasedmapcomponent))
        (`TimerComponent.SetTimer` _matchtimer _output_phaselength)
        (`TimerComponent.ResumeTimer` _matchtimer)))))

(event `self.SpawnRequestPublisher.OnSpawnRequest`
  (params (Controller :type "PlayerController Object Reference"))
  ;[1 1 1] Pass spawn requests to team spawner
  (`TeamSpawnerComponent.RequestSpawn` (`self.TeamSpawner`) Controller))

(event `self.MatchTimer.OnTimerFinished`
  ;[1 1 1] Finish Timer
  (`/Engine/EditorBlueprintResources/ActorMacros.Switch Has Authority`
    (:`Authority`
      (`/Game/GameMode/Components/PhaseBasedMapComponent.IncrementPhase` (`self.PhaseBasedMapComponent`))
      (set `TeamSpawnerComponent.bAllowRespawning` false (`self.TeamSpawner`)))))

(event `EvaluateWinCondition`
  (bind _phasebasedmapcomponent (`self.PhaseBasedMapComponent`))
  ;[1 1 1] Finish Timer
  (if (and (<= (`/Game/GameMode/Components/SquadTrackingComponent.AliveSquads` (`self.SquadTrackingComponent`)) 1) (> (`/Game/GameMode/Components/PhaseBasedMapComponent.CurrentPhase` _phasebasedmapcomponent) 0) (`/Game/GameMode/Components/PhaseBasedMapComponent.IsInFinalPhase` _phasebasedmapcomponent) (`|EnumEquality` (`MatchStateComponent.GetCurrentState` (`self.MatchState`)) "InGame"))
    (`MatchStateComponent.SetMatchState` (`self.MatchState`) "PostGame")
    (`/Game/GameMode/Components/SquadTrackingComponent.SetAllowWinningTeam` (`self.SquadTrackingComponent`) true)))

(fn `UserConstructionScript`)