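; BP_Bulkhead is a corridor shooter door made of three bulkhead meshes that opens and closes.
; OnOpen and OnClose play and reverse a timeline whose value slides two panels apart along Y while the third moves along Z.
; SnapOpen and SnapClosed set a forced time on that timeline to jump to either state.
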(event `self.OnOpen`
  (bind (_direction _dooropenvalue) (`Timeline|DoorTimeline` :`NewTime` (`self.ForcedDoorTime`) :!label _label)
    (:`Update`
      (`SceneComponent.K2_SetRelativeLocation` (`self.SM_General_Bulkhead_c03`) (`KismetMathLibrary.MakeVector` 0.0 0.0 (* _dooropenvalue 50.0)) false false)
      (`SceneComponent.K2_SetRelativeLocation` (`self.SM_General_Bulkhead_c01`) (`KismetMathLibrary.MakeVector` 0.0 (* _dooropenvalue -200.0)) false false)
      (`SceneComponent.K2_SetRelativeLocation` (`self.SM_General_Bulkhead_c02`) (`KismetMathLibrary.MakeVector` 0.0 (* _dooropenvalue 200.0)) false false))))

(event `self.OnClose`
  (goto _label :!via `Reverse`))

(event `self.SnapOpen`
  (set `self.ForcedDoorTime` 1.5)
  (goto _label :!via `SetNewTime`))

(event `self.SnapClosed`
  (set `self.ForcedDoorTime` 0.0)
  (goto _label :!via `SetNewTime`))

(fn `UserConstructionScript`)